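; Player controller that handles the inventory screen and on-screen subtitles.
; On BeginPlay it adds the default Enhanced Input mapping context and pre-creates the inventory widget.
; The inventory action flip-flops the widget in and out of the viewport, toggling the mouse cursor and pawn input; the input-mode switches are left unconnected.
; Separate functions create a subtitle widget with given text and remove it.
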(event `self.ReceiveBeginPlay`
  (bind _returnvalue (subsystem `EnhancedInputLocalPlayerSubsystem`))
  (`/Engine/EditorBlueprintResources/StandardMacros.IsValid` _returnvalue
    (:`Is Valid`
      (`EnhancedInputSubsystemInterface.AddMappingContext` _returnvalue "/Game/FirstPerson/Input/IMC_Default.IMC_Default" 0 (struct))
      (bind _returnvalue_2 (`|CreateWidget` "/MyContents/MyContents/InventorySystem/WG_Inventory.WG_Inventory_C"))
      (set `self.InventoryWidget` _returnvalue_2))))

(event `EnhancedInput|/Game/FirstPerson/Input/Actions/IA_Inventory`
  (params (ActionValue :type Boolean) (ElapsedSeconds :type "Float (double-precision)") (TriggeredSeconds :type "Float (double-precision)") (InputAction :type "InputAction Object Reference" :default "/Game/FirstPerson/Input/Actions/IA_Inventory.IA_Inventory"))
  (:`Started`
    (`/Engine/EditorBlueprintResources/StandardMacros.FlipFlop`
      (:`A`
        (`self.InventoryOpen`))
      (:`B`
        (`self.InventoryClose`)))))

(fn `CreateSubtitle`
  (params (text :type String))
  (bind _returnvalue (`|CreateWidget` "/Game/MyContents/Widgets/WG_Subtitle.WG_Subtitle_C" null text))
  (`UserWidget.AddToViewport` _returnvalue 0)
  (set `self.Subtitle` _returnvalue))

(fn `InventoryClose`
  (`Widget.RemoveFromParent` (`self.InventoryWidget`))
  (set `self.bShowMouseCursor` false)
  (`self.EnableInput` (`GameplayStatics.GetPlayerPawn` 0) null))

(fn `InventoryOpen`
  (`UserWidget.AddToViewport` (`self.InventoryWidget`) 0)
  (set `self.bShowMouseCursor` true)
  (`self.DisableInput` (`GameplayStatics.GetPlayerPawn` 0) null))

(fn `RemoveSubtitle`
  (`Widget.RemoveFromParent` (`self.Subtitle`)))

(fn `UserConstructionScript`)