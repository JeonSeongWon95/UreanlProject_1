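; BP_EnemyController is an enemy AI controller that caches the player pawn on BeginPlay and runs BT_enemy.
; Perception updates go to CheckPlayerSight, which sets or clears the Player blackboard key and saves LastKnowLocation when sight is lost.
; CheckPlayerSound writes heard stimulus locations to ReasoningLocation, but the event graph does not call it.
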(event `self.ReceiveBeginPlay`
  (bind _asbp_player (cast `/Game/MyContents/BluePrint/BP_Player` (`self.K2_GetPawn` (`GameplayStatics.GetPlayerController` 0))))
  (set `self.Player` _asbp_player)
  (`self.RunBehaviorTree` "/Game/MyContents/BluePrint/Enemy/BT_enemy.BT_enemy"))

(event `self.AIPerception.OnTargetPerceptionUpdated`
  (params (Actor :type "Actor Object Reference") (Stimulus :type "AIStimulus Structure"))
  (`self.CheckPlayer(Sight)` Actor Stimulus))

(fn `CheckPlayer(Sight)`
  (params (Player :type "Actor Object Reference") (Stimulus :type "AIStimulus Structure"))
  (bind (_age _expirationage _strength _stimuluslocation _receiverlocation _tag _bsuccessfullysensed) (break `AIStimulus` Stimulus))
  (bind _returnvalue (`AIPerceptionSystem.GetSenseClassForStimulus` Stimulus))
  (if (== _returnvalue "/Script/AIModule.AISense_Sight")
    (if (== Player (`self.Player`))
      (`BlackboardComponent.SetValueAsObject` (`AIBlueprintHelperLibrary.GetBlackboard` null) "Player" (`KismetMathLibrary.SelectObject` (`self.Player`) null _bsuccessfullysensed))
      (if (not _bsuccessfullysensed)
        (`BlackboardComponent.SetValueAsVector` (`AIBlueprintHelperLibrary.GetBlackboard` null) "LastKnowLocation" _stimuluslocation)))))

(fn `CheckPlayer(Sound)`
  (params (Stimulus :type "AIStimulus Structure"))
  (bind _returnvalue (`AIPerceptionSystem.GetSenseClassForStimulus` Stimulus))
  (if (== _returnvalue "/Script/AIModule.AISense_Hearing")
    (`BlackboardComponent.SetValueAsVector` (`AIBlueprintHelperLibrary.GetBlackboard` null) "ReasoningLocation" (`.StimulusLocation` (break `AIStimulus` Stimulus)))))

(fn `UserConstructionScript`)