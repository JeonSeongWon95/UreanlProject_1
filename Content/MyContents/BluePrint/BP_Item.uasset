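; BP_Item is a pickup item actor that the player collects into their inventory through interaction.
; The construction script looks up its RowName in DT_ItemTable, stores the row as Data and applies that row's static mesh.
; The Interaction override calls the parent, adds Data to the player pawn's BP_InventoryComponent, then destroys the actor.
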(fn `Interaction`
  (`parent.Interaction`)
  (`/MyContents/MyContents/InventorySystem/BP_InventoryComponent.AddItem` (`self.GetComponentByClass` (`GameplayStatics.GetPlayerPawn` 0) "/MyContents/MyContents/InventorySystem/BP_InventoryComponent.BP_InventoryComponent_C") (`self.Data`))
  (`self.K2_DestroyActor`))

(fn `UserConstructionScript`
  (`parent.UserConstructionScript`)
  (bind _returnvalue (`|GetDataTableRow` "/MyContents/MyContents/InventorySystem/DT_ItemTable.DT_ItemTable" (`self.Row Name`))
    (:`then`
      (bind _output_get (set `self.Data` _returnvalue))
      (`StaticMeshComponent.SetStaticMesh` (`self.StaticMesh`) (`.StaticMesh_9_81DABB8F42DBD3C6A3A642A640115F6E` (break `/MyContents/MyContents/InventorySystem/ST_Item` _output_get))))))