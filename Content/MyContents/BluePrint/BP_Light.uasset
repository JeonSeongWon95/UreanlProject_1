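; BP_Light is a blinking light actor with sound, a non-item child of a parent class that provides StartStep.
; Construction sets the light color, and BeginPlay loops BlinkLight, which schedules OffLight and OnLight after configurable delays.
; The StartStep override raises intensity far above the blink level and schedules EndStep, which is not defined here.
; Each on/off change plays audio, including EndLight, which nothing here calls.
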(event `self.ReceiveBeginPlay`
  (`parent.ReceiveBeginPlay`)
  (`KismetSystemLibrary.K2_SetTimer` null "BlinkLight" 6.0 true))

(fn `BlinkLight`
  (`KismetSystemLibrary.K2_SetTimer` null "OffLight" (`self.EndTime`))
  (`KismetSystemLibrary.K2_SetTimer` null "OnLight" (`self.StartTime`)))

(fn `EndLight`
  (`LightComponent.SetIntensity` (`self.PointLight`) 0.0)
  (`AudioComponent.Play` (`self.Audio`) 0.0))

(fn `OffLight`
  (`AudioComponent.Play` (`self.Audio`) 0.0)
  (`LightComponent.SetIntensity` (`self.PointLight`) 0.0))

(fn `OnLight`
  (`AudioComponent.Play` (`self.Audio`) 0.0)
  (`LightComponent.SetIntensity` (`self.PointLight`) 1500.0))

(fn `StartStep`
  (`parent.StartStep`)
  (`LightComponent.SetIntensity` (`self.PointLight`) 100000.0)
  (`AudioComponent.Play` (`self.Audio`) 0.0)
  (`KismetSystemLibrary.K2_SetTimer` null "EndStep" 6.0))

(fn `UserConstructionScript`
  (`parent.UserConstructionScript`)
  (set `self.IsItem` false)
  (`LightComponent.SetLightColor` (`self.PointLight`) (`self.New Light Color`) true))