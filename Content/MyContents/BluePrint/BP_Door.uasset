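; Door actor that slides upward with a sound when OpenDoor is called and IsOpenDoor is true.
; The construction script clears IsItem and sets the open height relative to the door mesh's starting world Z.
; OpenDoor starts a looping timer that calls MoveDoor to nudge the mesh up along local Z until it passes that height.
; The file never clears the timer or closes the door.
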(fn `MoveDoor`
  (bind _door (`self.Door`))
  (bind (_returnvalue_x _returnvalue_y _returnvalue_z) (`KismetMathLibrary.BreakVector` (`SceneComponent.K2_GetComponentLocation` _door)))
  (if (<= _returnvalue_z (`self.OpenPosition`))
    (`SceneComponent.K2_AddLocalOffset` _door (0.0 0.0 0.5) false false)))

(fn `OpenDoor`
  (if (`self.IsOpenDoor`)
    (`AudioComponent.Play` (`self.Audio`) 0.0)
    (`KismetSystemLibrary.K2_SetTimer` null "MoveDoor" 0.01 true)))

(fn `UserConstructionScript`
  (bind (_returnvalue_x _returnvalue_y _returnvalue_z) (`KismetMathLibrary.BreakVector` (`SceneComponent.K2_GetComponentLocation` (`self.Door`))))
  (`parent.UserConstructionScript`)
  (set `self.IsItem` false)
  (set `self.OpenPosition` (+ _returnvalue_z 240.0)))