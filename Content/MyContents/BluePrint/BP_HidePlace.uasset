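; BP_HidePlace is an interactable locker that the player can hide in, using a closed-locker static mesh set in the construction script.
; Its Interaction override toggles the player's IsHide state, teleporting them between inside and outside position markers and disabling movement while hidden through IsMove.
; Each toggle plays audio and starts a held camera fade to full alpha, with no fade back in this Blueprint.
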(fn `Interaction`
  (bind _player (`self.Player`))
  (bind _player_2 (`self.Player`))
  (`parent.Interaction`)
  (if (`/Game/MyContents/BluePrint/BP_Player.IsHide` (`self.Player`))
    (`AudioComponent.Play` (`self.Audio`) 0.0)
    (`PlayerCameraManager.StartCameraFade` :`self` (`GameplayStatics.GetPlayerCameraManager` 0) :`ToAlpha` 1.0 :`bHoldWhenFinished` true)
    (`self.K2_SetActorLocation` (`self.Player`) (`SceneComponent.K2_GetComponentLocation` (`self.OutPlayerPosition`)) false false)
    (set `/Game/MyContents/BluePrint/BP_Player.IsMove` true _player)
    (set `/Game/MyContents/BluePrint/BP_Player.IsHide` false _player)
    (else
      (`AudioComponent.Play` (`self.Audio`) 0.0)
      (`PlayerCameraManager.StartCameraFade` :`self` (`GameplayStatics.GetPlayerCameraManager` 0) :`ToAlpha` 1.0 :`bHoldWhenFinished` true)
      (`self.K2_SetActorLocation` (`self.Player`) (`SceneComponent.K2_GetComponentLocation` (`self.InPlayerPosition`)) false false)
      (set `/Game/MyContents/BluePrint/BP_Player.IsMove` false _player_2)
      (set `/Game/MyContents/BluePrint/BP_Player.IsHide` true _player_2))))

(fn `UserConstructionScript`
  (`parent.UserConstructionScript`)
  (`StaticMeshComponent.SetStaticMesh` (`self.StaticMesh`) "/MyMap/ModularSciFi/StaticMeshes/HardSurfaceEnvironment/Locker/SM_Locker_Closed.SM_Locker_Closed"))