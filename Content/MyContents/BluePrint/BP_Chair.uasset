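; BP_Chair is an interactable chair that lets the player sit on it.
; It overrides the Interaction function of its parent class, calls the parent, then casts the controlled pawn to BP_Player and calls Sit with the static mesh's world location.
; It then clears the IsHit flag; BeginPlay and the construction script only call their parent versions.
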(event `self.ReceiveBeginPlay`
  (`parent.ReceiveBeginPlay`))

(fn `Interaction`
  (`parent.Interaction`)
  (bind _asbp_player (cast `/Game/MyContents/BluePrint/BP_Player` (`Controller.K2_GetPawn` (`GameplayStatics.GetPlayerController` 0))))
  (`/Game/MyContents/BluePrint/BP_Player.Sit` _asbp_player (`SceneComponent.K2_GetComponentLocation` (`self.StaticMesh`)))
  (set `self.IsHit` false))

(fn `UserConstructionScript`
  (`parent.UserConstructionScript`))