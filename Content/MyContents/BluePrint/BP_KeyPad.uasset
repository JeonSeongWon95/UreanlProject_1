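; BP_KeyPad is an interactable keypad that opens its linked door when the player has the matching key item selected.
; Its Interaction override calls the parent, then compares the selected item's type on BP_Player against its own key type.
; On a match with a valid Door, it opens the door, uses the item, swaps a mesh material to a different display and clears IsHit.
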(fn `Interaction`
  (bind _mykeytype_itemtype (break `/MyContents/MyContents/InventorySystem/ST_Item` (`self.MyKeyType`)))
  (`parent.Interaction`)
  (bind _asbp_player (cast `/Game/MyContents/BluePrint/BP_Player` (`GameplayStatics.GetPlayerPawn` 0)))
  (bind _selectitem (`/Game/MyContents/BluePrint/BP_Player.SelectItem` _asbp_player)
    (:`then`
      (bind _data_itemtype (break `/MyContents/MyContents/InventorySystem/ST_Item` (`/Game/MyContents/BluePrint/BP_Item.Data` _selectitem)))
      (if (`|EnumEquality` _data_itemtype _mykeytype_itemtype)
        (bind _door (`self.Door`)
          (:`then`
            (`/Game/MyContents/BluePrint/BP_Door.OpenDoor` _door)
            (`/Game/MyContents/BluePrint/BP_Player.UseItem` _asbp_player)
            (`PrimitiveComponent.SetMaterial` (`self.StaticMesh`) 1 "/Game/ModularSciFi/Materials/Display/MI_Dispalay_3.MI_Dispalay_3")
            (set `self.IsHit` false))
          (:`else`))))
    (:`else`)))

(fn `UserConstructionScript`
  (`parent.UserConstructionScript`))