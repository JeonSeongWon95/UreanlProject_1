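; BP_GuideSound is a guide step that plays a sound and ends when the audio finishes.
; It overrides StartStep to call the parent, assign Sound to the Audio component, play it and bind to its OnAudioFinished event.
; SoundFinishedStep calls EndStep to close the step, and the event graph holds only disabled default events.
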(fn `SoundFinishedStep`
  (`self.EndStep`))

(fn `StartStep`
  (`parent.StartStep`)
  (`AudioComponent.SetSound` (`self.Audio`) (`self.Sound`))
  (`AudioComponent.Play` (`self.Audio`) 0.0)
  (add `AudioComponent.OnAudioFinished` (`self.Audio`) (`|CreateDelegate` :!event `SoundFinishedStep`)))

(fn `UserConstructionScript`
  (`parent.UserConstructionScript`))