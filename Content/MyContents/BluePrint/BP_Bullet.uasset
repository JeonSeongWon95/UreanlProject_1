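; BP_Bullet is a sphere projectile that flies straight along its forward vector and expires after two seconds.
; A looping timer calls Flying, which offsets the actor by a fixed step without sweep, instead of using Tick or a movement component.
; The construction script sets the sphere mesh, copies it to a procedural mesh with collision and clears IsHit, though no hit handling is implemented here.
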(event `self.ReceiveBeginPlay`
  (`parent.ReceiveBeginPlay`)
  (`self.SetLifeSpan` 2.0)
  (`KismetSystemLibrary.K2_SetTimer` null "Flying" 0.01 true))

(fn `Flying`
  (`self.K2_AddActorWorldOffset` (* (`self.GetActorForwardVector`) 25.0)))

(fn `UserConstructionScript`
  (`parent.UserConstructionScript`)
  (`StaticMeshComponent.SetStaticMesh` (`self.StaticMesh`) "/Engine/EditorMeshes/ArcadeEditorSphere.ArcadeEditorSphere")
  (set `self.IsHit` false)
  (`KismetProceduralMeshLibrary.CopyProceduralMeshFromStaticMeshComponent` (`self.StaticMesh`) 0 (`self.ProceduralMesh`) true))