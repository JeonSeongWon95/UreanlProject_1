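; BP_CameraFadeIn is a step Blueprint that fades the player's camera in from a fully faded screen.
; StartStep calls the parent, then issues a full-opacity hold fade that is immediately replaced by a five-second fade to clear on player 0's camera manager.
; A timer set by function name calls EndStep when the fade duration elapses, and the event graph holds only disabled stubs.
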(fn `StartStep`
  (bind _returnvalue (`GameplayStatics.GetPlayerCameraManager` 0))
  (`parent.StartStep`)
  (`PlayerCameraManager.StartCameraFade` :`self` _returnvalue :`FromAlpha` 1.0 :`ToAlpha` 1.0 :`Duration` 5.0 :`bHoldWhenFinished` true)
  (`PlayerCameraManager.StartCameraFade` :`self` _returnvalue :`FromAlpha` 1.0 :`ToAlpha` 0.0 :`Duration` 5.0 :`bHoldWhenFinished` true)
  (`KismetSystemLibrary.K2_SetTimer` null "EndStep" 5.0))

(fn `UserConstructionScript`
  (`parent.UserConstructionScript`))