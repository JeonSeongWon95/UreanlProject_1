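; BP_Boss is an unfinished boss actor that breaks the BrokenWall entry at WallNumber on BeginPlay.
; Attacked checks Health, then either decrements it or calls the empty Die.
; ChangeAttackPattern picks a random pattern, using a second pool at 3 Health or below, but its timer in Attack is unreachable.
; Attack's switch on AttackPattern has no branches, and ElectricFloor is an empty stub.
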(event `self.ReceiveBeginPlay`
  (`self.BrakenWall`))

(fn `Attack`
  (switch `/Game/MyContents/BluePrint/EN_Pattern` (`self.AttackPattern`)))

(fn `Attacked`
  (if (<= (`self.Health`) 0)
    (`self.Die`)
    (else
      (set `self.Health` (- (`self.Health`) 1)))))

(fn `BrakenWall`
  (`/Game/MyContents/BluePrint/BP_Wall.Broken` (`|GetArrayItem` (`self.BrokenWall`) (`self.WallNumber`))))

(fn `ChangeAttackPattern`
  (if (<= (`self.Health`) 3)
    (set `self.AttackPattern` (`KismetArrayLibrary.Array_Random` (`self.AttackPatterns2`)))
    (else
      (set `self.AttackPattern` (`KismetArrayLibrary.Array_Random` (`self.AttackPatterns`))))))

(fn `Die`)

(fn `Electric Floor`)

(fn `UserConstructionScript`)