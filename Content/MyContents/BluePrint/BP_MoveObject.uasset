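; BP_MoveObject is an interactable physics object the player can pick up and release when holding no selected item.
; Interaction toggles IsSelect, switching IsHit, the player's line trace and the widget.
; While carried, a fast looping SetLocation timer, used instead of Tick, keeps it at a fixed distance ahead of the player.
; Physics starts on at BeginPlay; any interaction disables it, and release does not restore it.
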(event `self.ReceiveBeginPlay`
  (`parent.ReceiveBeginPlay`)
  (`PrimitiveComponent.SetSimulatePhysics` (`self.StaticMesh`) true))

(fn `Interaction`
  (`parent.Interaction`)
  (`PrimitiveComponent.SetSimulatePhysics` (`self.StaticMesh`) false)
  (bind _asbp_player (cast `/Game/MyContents/BluePrint/BP_Player` (`GameplayStatics.GetPlayerPawn` 0)))
  (`/Game/MyContents/BluePrint/BP_Player.SelectItem` _asbp_player
    (:`then`)
    (:`else`
      (if (`self.IsSelect`)
        (set `self.IsHit` false)
        (bind _asbp_player_2 (cast `/Game/MyContents/BluePrint/BP_Player` (`GameplayStatics.GetPlayerPawn` 0)))
        (bind _output_get (set `/Game/MyContents/BluePrint/BP_Player.IsLineTraceOn` false _asbp_player_2))
        (`self.SetWidget` _output_get)
        (set `self.IsSelect` false)
        (`KismetSystemLibrary.K2_SetTimer` null "SetLocation" 0.01 true)
        (else
          (`KismetSystemLibrary.K2_ClearTimer` null "SetLocation")
          (set `self.IsHit` true)
          (bind _asbp_player_3 (cast `/Game/MyContents/BluePrint/BP_Player` (`GameplayStatics.GetPlayerPawn` 0)))
          (bind _output_get_2 (set `/Game/MyContents/BluePrint/BP_Player.IsLineTraceOn` true _asbp_player_3))
          (`self.SetWidget` _output_get_2)
          (set `self.IsSelect` true))))))

(fn `SetLocation`
  (bind _returnvalue (`GameplayStatics.GetPlayerPawn` 0))
  (`self.K2_SetActorLocation` (+ (`self.K2_GetActorLocation` _returnvalue) (* (`self.GetActorForwardVector` _returnvalue) 300.0))))

(fn `UserConstructionScript`
  (`parent.UserConstructionScript`))