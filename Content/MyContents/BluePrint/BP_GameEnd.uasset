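; BP_GameEnd is an interactable actor that ends the game when used.
; It flags itself as an item on BeginPlay and overrides the parent's Interaction.
; Interaction fades the player camera out over a short duration and holds it, then calls ShowGameEnd on BP_PlayerController without waiting for the fade to finish.
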(event `self.ReceiveBeginPlay`
  (`parent.ReceiveBeginPlay`)
  (set `self.IsItem` true))

(fn `Interaction`
  (`parent.Interaction`)
  (`PlayerCameraManager.StartCameraFade` :`self` (`GameplayStatics.GetPlayerCameraManager` 0) :`ToAlpha` 1.0 :`Duration` 2.0 :`bHoldWhenFinished` true)
  (bind _asbp_player_controller (cast `/Game/MyContents/BluePrint/BP_PlayerController` (`GameplayStatics.GetPlayerController` 0)))
  (`/Game/MyContents/BluePrint/BP_PlayerController.ShowGameEnd` _asbp_player_controller))

(fn `UserConstructionScript`
  (`parent.UserConstructionScript`))