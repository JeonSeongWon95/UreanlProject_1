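; Opening-level spotlight actor that blinks on and off with sound, changing a displayed static mesh between flashes.
; A looping timer calls On, which sets an emissive material, lights the spot and schedules Off.
; Off restores the stand material, kills the light and picks a random mesh from Meshs while dark.
; The StartStep override raises intensity sharply and schedules EndStep, while EndLight separately cuts the light with sound.
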(event `self.ReceiveBeginPlay`
  (`parent.ReceiveBeginPlay`)
  (`KismetSystemLibrary.K2_SetTimer` null "On" 5.0 true))

(fn `EndLight`
  (`LightComponent.SetIntensity` (`self.Spot`) 0.0)
  (`AudioComponent.Play` (`self.Audio`) 0.0))

(fn `Off`
  (`AudioComponent.Play` (`self.Audio`) 0.0)
  (`PrimitiveComponent.SetMaterial` (`self.Light`) 0 "/Light/BigStarStation/Materials/MI_StandLight.MI_StandLight")
  (`StaticMeshComponent.SetStaticMesh` (`self.StaticMesh`) (`|GetArrayItem` (`self.Meshs`) (`KismetMathLibrary.RandomInteger` 10)))
  (`LightComponent.SetIntensity` (`self.Spot`) 0.0))

(fn `On`
  (`PrimitiveComponent.SetMaterial` (`self.Light`) 0 "/Light/BigStarStation/Materials/MI_LightEmissive.MI_LightEmissive")
  (`AudioComponent.Play` (`self.Audio`) 0.0)
  (`LightComponent.SetIntensity` (`self.Spot`) 5000.0)
  (`KismetSystemLibrary.K2_SetTimer` null "Off" 4.0))

(fn `StartStep`
  (`parent.StartStep`)
  (`LightComponent.SetIntensity` (`self.Spot`) 100000.0)
  (`AudioComponent.Play` (`self.Audio`) 0.0)
  (`KismetSystemLibrary.K2_SetTimer` null "EndStep" 5.0))

(fn `UserConstructionScript`
  (`parent.UserConstructionScript`))